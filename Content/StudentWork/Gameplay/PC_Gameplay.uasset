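; PC_Gameplay is the gameplay player controller, holding a PlayerData struct with team ID and gating input by match phase.
; Init binds to GS_MyGameState's state-change event, enabling player controller 0's input in In Game and disabling it in Setup, Pre and Post Game.
; Setters and getters expose PlayerData and its team.
; The M key removes all players and opens the MainMenu level.
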(event Custom|Init
  (EventDispatchers|BindEventtoGameStateChanged (.AsGS%20My%20Game%20State (Utilities|Casting|CastToGS_MyGameState (Game|GetGameState))) (EventDispatchers|CreateEvent :!event Custom|GameStateChanged)))

(event Custom|GameStateChanged
  (params (CurrentGameState :type E_GameState%20Enum :default "NewEnumerator0"))
  (bind _returnvalue (Game|GetPlayerController 0))
  (bind _self self)
  (Development|PrintString "Changed")
  (switch Utilities|FlowControl|Switch|SwitchonE_GameState CurrentGameState
    (:NewEnumerator0
      (Input|DisableInput _returnvalue _self :!label _label))
    (:NewEnumerator1
      (goto _label))
    (:NewEnumerator2
      (Input|EnableInput _returnvalue _self))
    (:NewEnumerator3
      (goto _label))))

(event EventBeginPlay
  (Development|PrintString "PC Gameplay"))

(event EventSetTeam
  (params (TeamID :type E_Teams%20Enum :default "NewEnumerator0"))
  (Utilities|Struct|SetmembersinS_PlayerData (Variables|Default|GetPlayer%20Data) TeamID))

(event EventSetPlayerData
  (params (playerData :type S%20Player%20Data%20Structure))
  (Variables|Default|SetPlayer%20Data playerData))

(event Input|KeyboardEvents|M
  (params (Key :type Key%20Structure :default "None"))
  (:Pressed
    (CallFunction|RemoveAllPlayers)
    (Game|OpenLevel(byName) "MainMenu")))

(fn ConstructionScript)

(fn GetPlayerData
  (return (Variables|Default|GetPlayer%20Data)))

(fn GetTeam
  (return (Utilities|Struct|BreakS_PlayerData (Variables|Default|GetPlayer%20Data))))