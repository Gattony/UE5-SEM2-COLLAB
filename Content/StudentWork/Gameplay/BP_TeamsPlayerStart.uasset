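; BP_TeamsPlayerStart is a team-tagged player start that stores a TeamID of No Team, Team A or Team B.
; Its construction script sets a text render's label and color from that ID, so the assignment is visible on placed instances.
; SetTeam writes the ID without refreshing the text, and GetTeam returns it.
; GetPlayerData is an empty stub.
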(event EventBeginPlay)

(event EventTick
  (params (DeltaSeconds :type Float%20%28single-precision%29)))

(event EventSetTeam
  (params (TeamID :type E_Teams%20Enum :default "NewEnumerator0"))
  (Variables|Default|SetTeamID TeamID))

(fn ConstructionScript
  (switch Utilities|FlowControl|Switch|SwitchonE_Teams (Variables|Default|GetTeamID)
    (:NewEnumerator0
      (Rendering|Components|TextRender|SetText (Variables|Default|GetTextRender) (Utilities|Text|MakeLiteralText "No Team")))
    (:NewEnumerator1
      (Rendering|Components|TextRender|SetText (Variables|Default|GetTextRender) (Utilities|Text|MakeLiteralText "Team A")))
    (:NewEnumerator2
      (Rendering|Components|TextRender|SetText (Variables|Default|GetTextRender) (Utilities|Text|MakeLiteralText "Team B"))))
  (Rendering|Components|TextRender|SetTextRenderColor (Variables|Default|GetTextRender) (Utilities|Select :Index (Variables|Default|GetTeamID) :NewEnumerator0 (Math|Color|MakeColor 255 255 255) :NewEnumerator1 (Math|Color|MakeColor 255) :NewEnumerator2 (Math|Color|MakeColor 255))))

(fn GetPlayerData
  (return ""))

(fn GetTeam
  (return (Variables|Default|GetTeamID)))