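; Team-based game mode (GM_TDM) for local multiplayer matches.
; On BeginPlay it creates a player for each active slot in the GameInstance's player data, sorts them into team lists and possesses their chosen characters at random team start points.
; It drives GameState from PreGame to SetupGame and reacts to state changes through a bound event.
; End checks switch to PostGame; a separate EndGame event removes players and opens MainMenu.
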(event Custom|Init
  (CallFunction|SetUpControllersGI)
  (CallFunction|SpawnCharacters)
  (CallFunction|BindtoGameState)
  (Default|Init (Variables|Default|GetAll%20Players))
  (Utilities|FlowControl|Delay 0.2)
  (Default|UpdateState (Variables|Default|GetGS%20Game%20State) "NewEnumerator1"))

(event Custom|BindToGameState
  (bind _output_get (Variables|Default|SetGS%20Game%20State (.AsGS%20My%20Game%20State (Utilities|Casting|CastToGS_MyGameState (Game|GetGameState)))))
  (EventDispatchers|BindEventtoGameStateChanged _output_get (EventDispatchers|CreateEvent :!event Custom|GameStateChanged)))

(event Custom|GameStateChanged
  (params (CurrentGameState :type E_GameState%20Enum :default "NewEnumerator0"))
  (switch Utilities|FlowControl|Switch|SwitchonE_GameState CurrentGameState
    (:NewEnumerator1
      (Development|PrintString "PreGame")
      (Utilities|FlowControl|Delay 0.2)
      (Default|UpdateState (Variables|Default|GetGS%20Game%20State) "NewEnumerator0"))
    (:NewEnumerator2
      (Development|PrintString "InGame")
      (Utilities|Time|SetTimerbyEvent (EventDispatchers|CreateEvent :!event Custom|TimeUp) 0.0))
    (:NewEnumerator3
      (Development|PrintString "PostGame"))))

(event Custom|TimeUp
  (Variables|Default|SetHasTimeRunOut true)
  (CallFunction|CanEndGame))

(event Custom|EndGame
  (Utilities|FlowControl|Delay 0.2)
  (CallFunction|RemoveAllPlayers)
  (Game|OpenLevel(byName) "MainMenu"))

(event EventBeginPlay
  ;[1 1 1] Get GI
  (Development|PrintString "GM DM")
  (Variables|Default|SetGameInstance (.AsGI%20Game%20Instance (Utilities|Casting|CastToGI_GameInstance (Game|GetGameInstance))))
  (CallFunction|Init))

(event EventPostLogin
  (params (NewPlayer :type Player%20Controller%20Object%20Reference))
  (bind _aspc_gameplay (Utilities|Casting|CastToPC_Gameplay NewPlayer))
  (Utilities|Array|Add (Variables|Default|GetAll%20Players) _aspc_gameplay))

(event EventOnLogout
  (params (ExitingController :type Controller%20Object%20Reference))
  (bind _aspc_gameplay (Utilities|Casting|CastToPC_Gameplay ExitingController))
  (Utilities|Array|RemoveItem (Variables|Default|GetAll%20Players) _aspc_gameplay))

(fn ConstructionScript)

(fn SetUpControllers
  (params (Number%20of%20Players :type Integer))
  (Class|GameplayStatics|RemovePlayer (Game|GetPlayerController 0) true)
  (for _index (range 0 (- Number%20of%20Players 1))
    (bind _returnvalue (Class|GameplayStatics|CreatePlayer _index))
    (Utilities|FlowControl|FlipFlop
      (:A
        (Class|BPITeams|SetTeam(Message) _returnvalue "NewEnumerator1"))
      (:B
        (Class|BPITeams|SetTeam(Message) _returnvalue "NewEnumerator2")))
    (CallFunction|AddtoTeamList (.AsPC%20Gameplay (Utilities|Casting|CastToPC_Gameplay _returnvalue)))))

(fn SpawnCharacters
  (for _array_element (Variables|Default|GetAll%20Players)
    (bind _playerdata (Class|BPITeams|GetPlayerData(Message) _array_element))
    (bind _returnvalue (Game|SpawnActorfromClass (.PlayerClass (Utilities|Struct|BreakS_PlayerData _playerdata)) (Transformation|GetActorTransform (CallFunction|SelectPlayerStart (.TeamID (Utilities|Struct|BreakS_PlayerData _playerdata)))) "AdjustIfPossibleButAlwaysSpawn" "MultiplyWithRoot" 0 0))
    (Pawn|Possess _array_element (.AsPawn (Utilities|Casting|CastToPawn _returnvalue)))))

(fn SelectPlayerStart
  (params (teamID :type E_Teams%20Enum :default "NewEnumerator0"))
  (bind _outactors (Actor|GetAllActorsOfClass "/Game/StudentWork/Gameplay/BP_TeamsPlayerStart.BP_TeamsPlayerStart_C"))
  (for _array_element _outactors
    (bind _teamid (Class|BPITeams|GetTeam(Message) _array_element))
    ;[1 1 1] Check and add to potential spawn points
    (if (Utilities|Enum|Equal(Enum) _teamid teamID)
      (Utilities|Array|Add (LocalVariables|GetL_SpawnPointActors) _array_element)))
  ;[1 1 1] Emergency Fallback
  (if (== (Utilities|Array|Length (LocalVariables|GetL_SpawnPointActors)) 0)
    (Development|PrintString "No Spawn points found" true true "(R=1.000000,G=0.000000,B=0.025978,A=1.000000)" 1e+01)
    (bind _outactors_2 (Actor|GetAllActorsOfClass "/Game/StudentWork/Gameplay/BP_TeamsPlayerStart.BP_TeamsPlayerStart_C"))
    (return (.OutItem (Utilities|Array|Random _outactors_2)))
    (else
      ;[1 1 1] Pick Random Team Start Point
      (return (.OutItem (Utilities|Array|Random (LocalVariables|GetL_SpawnPointActors)))))))

(fn AddtoTeamList
  (params (Gameplay%20Controllers :type PC%20Gameplay%20Object%20Reference))
  (bind _teamid (Class|BPITeams|GetTeam(Message) Gameplay%20Controllers))
  (switch Utilities|FlowControl|Switch|SwitchonE_Teams _teamid
    (:NewEnumerator1
      (Utilities|Array|Add (Variables|Default|GetTeamA_Players) Gameplay%20Controllers))
    (:NewEnumerator2
      (Utilities|Array|Add (Variables|Default|GetTeamB_Players) Gameplay%20Controllers))))

(fn SetUpControllersGI
  (bind _gameinstance (Variables|Default|GetGameInstance))
  (Class|GameplayStatics|RemovePlayer (Game|GetPlayerController 0) true)
  (for _index (range 0 3)
    (if (.isActive (Utilities|Struct|BreakS_PlayerData (Utilities|Select :Index _index :Option%200 (Variables|/Game/StudentWork/Gameplay/GI_GameInstance.GI_GameInstance_C|GetPlayer0_data _gameinstance) :Option%201 (Variables|/Game/StudentWork/Gameplay/GI_GameInstance.GI_GameInstance_C|GetPlayer1_data _gameinstance) :Option%202 (Variables|/Game/StudentWork/Gameplay/GI_GameInstance.GI_GameInstance_C|GetPlayer2_data _gameinstance) :Option%203 (Variables|/Game/StudentWork/Gameplay/GI_GameInstance.GI_GameInstance_C|GetPlayer3_data _gameinstance))))
      (bind _returnvalue (Class|GameplayStatics|CreatePlayer (.PlayerID (Utilities|Struct|BreakS_PlayerData (Utilities|Select :Index _index :Option%200 (Variables|/Game/StudentWork/Gameplay/GI_GameInstance.GI_GameInstance_C|GetPlayer0_data _gameinstance) :Option%201 (Variables|/Game/StudentWork/Gameplay/GI_GameInstance.GI_GameInstance_C|GetPlayer1_data _gameinstance) :Option%202 (Variables|/Game/StudentWork/Gameplay/GI_GameInstance.GI_GameInstance_C|GetPlayer2_data _gameinstance) :Option%203 (Variables|/Game/StudentWork/Gameplay/GI_GameInstance.GI_GameInstance_C|GetPlayer3_data _gameinstance))))))
      (Class|BPITeams|SetPlayerData(Message) _returnvalue (Utilities|Select :Index _index :Option%200 (Variables|/Game/StudentWork/Gameplay/GI_GameInstance.GI_GameInstance_C|GetPlayer0_data _gameinstance) :Option%201 (Variables|/Game/StudentWork/Gameplay/GI_GameInstance.GI_GameInstance_C|GetPlayer1_data _gameinstance) :Option%202 (Variables|/Game/StudentWork/Gameplay/GI_GameInstance.GI_GameInstance_C|GetPlayer2_data _gameinstance) :Option%203 (Variables|/Game/StudentWork/Gameplay/GI_GameInstance.GI_GameInstance_C|GetPlayer3_data _gameinstance)))
      (CallFunction|AddtoTeamList (.AsPC%20Gameplay (Utilities|Casting|CastToPC_Gameplay _returnvalue))))))

(fn CanEndGame
  (if (Math|Boolean|ORBoolean (Variables|Default|GetHasTimeRunOut) (Variables|Default|GetHaveAllPlayersDied) (Variables|Default|GetHaveAllItemsBeenCollected))
    (Default|UpdateState (Variables|Default|GetGS%20Game%20State) "NewEnumerator3")))